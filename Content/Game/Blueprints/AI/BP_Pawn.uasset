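; BP_Pawn is an AI pawn that can be selected with a marquee.
; Marquee selection and deselection events show and hide its SelectionDecalComponent to mark the selected state.
; IsCurrentlySelectableByMarquee always returns true, regardless of the selecting player.
; BeginPlay, overlap and Tick are unused stubs, and the construction script only calls its parent.
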(event EventBeginPlay
  (|CallParentFunction) ; This node is disabled and will not be called.\nDrag off pins to build functionality.
)

(event Collision|EventActorBeginOverlap
  (params (OtherActor :type Actor%20Object%20Reference)))

(event EventTick
  (params (DeltaSeconds :type Float%20%28single-precision%29)))

(event EventOnSelectedbyMarquee
  (params (SelectingPlayer :type Player%20Controller%20Object%20Reference))
  (Rendering|SetVisibility (Variables|Default|GetSelectionDecalComponent) true false))

(event EventOnDeselectedbyMarquee
  (params (SelectingPlayer :type Player%20Controller%20Object%20Reference))
  (Rendering|SetVisibility (Variables|Default|GetSelectionDecalComponent) false false))

(fn ConstructionScript
  (|CallParentFunction))

(fn IsCurrentlySelectablebyMarquee
  (params (SelectingPlayer :type Player%20Controller%20Object%20Reference))
  (return true))