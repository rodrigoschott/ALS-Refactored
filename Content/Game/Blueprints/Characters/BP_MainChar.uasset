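; Main player character built on ALS, with abilities from the Gameplay Ability System.
; References caches the player state and its ability component at BeginPlay, letting inputs activate top-down view and marquee selection abilities.
; Overlay mode changes link the matching animation layer and attach held props to hand sockets or gun bones, with props cleared during non-low mantles and ragdoll.
; Debug prints report marquee activation and, on left click, base health.
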(event Input|EnhancedActionEvents|EnhancedInputActionIA_ToggleTopDownView
  (params (ActionValue :type Boolean) (ElapsedSeconds :type Float%20%28double-precision%29) (TriggeredSeconds :type Float%20%28double-precision%29) (InputAction :type Input%20Action%20Object%20Reference :default "/ALS/Game/Data/Input/TopDown/IA_ToggleTopDownView.IA_ToggleTopDownView"))
  (Abilities|TryActivateAbilitybyClass (Variables|References|GetAbilityComponentRef) "/ALS/Game/Blueprints/Abilities/GA_SetupAndControls/BGA_SetViewModeTopDown.BGA_SetViewModeTopDown_C" true))

(event Input|EnhancedActionEvents|EnhancedInputActionIA_MarqueeSelect_Hold
  (params (ActionValue :type Boolean) (ElapsedSeconds :type Float%20%28double-precision%29) (TriggeredSeconds :type Float%20%28double-precision%29) (InputAction :type Input%20Action%20Object%20Reference :default "/ALS/Game/Data/Input/TopDown/IA_MarqueeSelect_Hold.IA_MarqueeSelect_Hold"))
  (:Started
    (bind _returnvalue (Abilities|TryActivateAbilitybyClass (Variables|References|GetAbilityComponentRef) "/ALS/Game/Blueprints/Abilities/GA_SetupAndControls/BGA_SelectionMarquee.BGA_SelectionMarquee_C" true))
    (Development|PrintString (Utilities|String|ToString(Boolean) _returnvalue))))

(event EventBeginPlay
  (|CallParentFunction)
  (|References))

(event Collision|EventActorBeginOverlap
  (params (OtherActor :type Actor%20Object%20Reference)))

(event EventTick
  (params (DeltaSeconds :type Float%20%28single-precision%29)))

(event Input|MouseEvents|DebugKeyRightMouseButton
  (params (Key :type Key%20Structure :default "None") (ActionValue :type Input%20Action%20Value%20Structure)))

(event Input|MouseEvents|DebugKeyLeftMouseButton
  (params (Key :type Key%20Structure :default "None") (ActionValue :type Input%20Action%20Value%20Structure))
  (:Pressed
    (Development|PrintString (Utilities|String|ToString(Float) (.BaseValue (Utilities|Struct|BreakGameplayAttributeData (Variables|/Script/Game.MyAttributeSet_CoreVitality|GetHealth (Class|MyPlayerState|GetCoreVitalityAttributeSet (Variables|References|GetPlayerStateRef)))))))))

(fn ConstructionScript
  (|CallParentFunction))

(fn ClearOverlayObject
  (Components|StaticMesh|SetStaticMesh (Variables|Default|GetOverlayStaticMesh) 0)
  (Components|SkinnedMesh|SetSkinnedAssetandUpdate (Variables|Components|GetOverlaySkeletalMesh) 0 true)
  (Components|SkeletalMesh|SetAnimInstanceClass (Variables|Components|GetOverlaySkeletalMesh) 0))

(fn AttachOverlayObject
  (params (NewStaticMesh :type Static%20Mesh%20Object%20Reference) (NewSkeletalMesh :type Skeletal%20Mesh%20Object%20Reference) (NewAnimationClass :type Anim%20Instance%20Class%20Reference) (SocketName :type Name) (bUseLeftGunBone :type Boolean))
  (LocalVariables|SetResultSocketName (select (Variables|Overlay|GetbUseGunBoneForOverlayObjects) (select bUseLeftGunBone (Class|AlsConstants|HandLeftGunVirtualBoneName) (Class|AlsConstants|HandRightGunVirtualBoneName)) SocketName))
  (Utilities|FlowControl|Sequence
    (:then_0
      (Components|StaticMesh|SetStaticMesh (Variables|Default|GetOverlayStaticMesh) NewStaticMesh)
      (Transformation|AttachComponentToComponent (Variables|Default|GetOverlayStaticMesh) (Variables|Character|GetMesh) (LocalVariables|GetResultSocketName) "SnapToTarget" "SnapToTarget" "SnapToTarget" true))
    (:then_1
      (Components|SkinnedMesh|SetSkinnedAssetandUpdate (Variables|Components|GetOverlaySkeletalMesh) NewSkeletalMesh true)
      (Components|SkeletalMesh|SetAnimInstanceClass (Variables|Components|GetOverlaySkeletalMesh) NewAnimationClass)
      (Transformation|AttachComponentToComponent (Variables|Components|GetOverlaySkeletalMesh) (Variables|Character|GetMesh) (LocalVariables|GetResultSocketName) "SnapToTarget" "SnapToTarget" "SnapToTarget" true))))

(fn RefreshOverlayObject
  (|SwitchGameplayTag (Variables|Default|GetOverlayMode)
    (:Default
      (Overlay|ClearOverlayObject))
    (:Als.OverlayMode.Rifle
      (Overlay|AttachOverlayObject 0 "/ALS/Game/Art/Weapons/Rifle/SKM_Als_Rifle.SKM_Als_Rifle" 0 "Rifle" false))
    (:Als.OverlayMode.PistolOneHanded
      (Overlay|AttachOverlayObject 0 "/ALS/Game/Art/Weapons/Pistol/SKM_Als_Pistol.SKM_Als_Pistol" 0 "Pistol" false :!label _label))
    (:Als.OverlayMode.PistolTwoHanded
      (goto _label))
    (:Als.OverlayMode.Bow
      (Overlay|AttachOverlayObject 0 "/ALS/Game/Art/Weapons/Bow/SKM_Als_Bow.SKM_Als_Bow" "/ALS/Game/Art/Weapons/Bow/AB_Als_Bow.AB_Als_Bow_C" "Bow" true))
    (:Als.OverlayMode.Torch
      (Overlay|AttachOverlayObject "/ALS/Game/Art/Items/Torch/SM_Als_Torch.SM_Als_Torch" 0 0 "Torch" true))
    (:Als.OverlayMode.Binoculars
      (Overlay|AttachOverlayObject "/ALS/Game/Art/Items/Binoculars/SM_Als_Binoculars.SM_Als_Binoculars" 0 0 "Binoculars" false))
    (:Als.OverlayMode.Box
      (Overlay|AttachOverlayObject "/ALS/Game/Art/Items/Box/SM_Als_Box.SM_Als_Box" 0 0 "Box" false))
    (:Als.OverlayMode.Barrel
      (Overlay|AttachOverlayObject "/ALS/Game/Art/Items/Barrel/SM_Als_Barrel.SM_Als_Barrel" 0 0 "Barrel" true))))

(fn RefreshOverlayLinkedAnimationLayer
  (bind _mesh (Variables|Character|GetMesh))
  (LocalVariables|SetOverlayAnimationInstanceClass (.Value (Utilities|Map|Find (Variables|Overlay|GetOverlayAnimationInstanceClasses) (Variables|Default|GetOverlayMode))))
  (bind _overlayanimationinstanceclass (LocalVariables|GetOverlayAnimationInstanceClass)
    (:then
      (Components|SkeletalMesh|AnimationBlueprintLinking|LinkAnimClassLayers _mesh _overlayanimationinstanceclass))
    (:else
      (Components|SkeletalMesh|AnimationBlueprintLinking|LinkAnimClassLayers _mesh "/ALS/Game/Animations/AnimationInstances/Overlays/AB_Als_Default.AB_Als_Default_C"))))

(event Custom|CustomEvent
  (Overlay|RefreshOverlayObject))

(event EventOnOverlayModeChanged
  (params (PreviousOverlayMode :type Gameplay%20Tag%20Structure%20%28by%20ref%29))
  (Overlay|RefreshOverlayLinkedAnimationLayer)
  (Overlay|RefreshOverlayObject))

(event EventOnMantlingEnded
  (Overlay|RefreshOverlayObject))

(event EventOnRagdollingEnded
  (Overlay|RefreshOverlayObject))

(event EventOnMantlingStarted
  (params (Parameters :type Als%20Mantling%20Parameters%20Structure%20%28by%20ref%29))
  (if (Utilities|Enum|NotEqual(Enum) (.mantlingtype Parameters) "Low")
    (Overlay|ClearOverlayObject)))

(event EventOnRagdollingStarted
  (Overlay|ClearOverlayObject))