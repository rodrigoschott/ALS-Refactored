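; Player controller for the ALS (Advanced Locomotion System) game that drives the HUD, overlay mode menu and slow motion.
; On local BeginPlay it adds the UI input mapping, shows the HUD and creates the overlay menu.
; Holding the menu input shows that menu and slows time, previous/next inputs cycle the selection, and release applies it.
; Toggles control slomo and a UI-visible flag; time dilation only applies in standalone play.
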(event Input|EnhancedActionEvents|EnhancedInputActionIA_Als_OverlayModeMenu
  (params (ActionValue :type Boolean) (ElapsedSeconds :type Float%20%28double-precision%29) (TriggeredSeconds :type Float%20%28double-precision%29) (InputAction :type Input%20Action%20Object%20Reference :default "/ALS/Game/Data/Input/UI/IA_Als_OverlayModeMenu.IA_Als_OverlayModeMenu"))
  (if ActionValue
    (if (Variables|State|GetbSlomoActive)
      _
      (else
        (CallFunction|SetGlobalTimeDilation 0.35)))
    (UserInterface|Viewport|AddtoViewport (Variables|State|GetOverlayModeMenuWidget) 0)
    (else
      (if (Variables|State|GetbSlomoActive)
        _
        (else
          (CallFunction|SetGlobalTimeDilation 1.0)))
      (Default|ApproveOverlayMode (Variables|State|GetOverlayModeMenuWidget))
      (Widget|RemovefromParent (Variables|State|GetOverlayModeMenuWidget)))))

(event Input|EnhancedActionEvents|EnhancedInputActionIA_Als_NextOverlayMode
  (params (ActionValue :type Boolean) (ElapsedSeconds :type Float%20%28double-precision%29) (TriggeredSeconds :type Float%20%28double-precision%29) (InputAction :type Input%20Action%20Object%20Reference :default "/ALS/Game/Data/Input/UI/IA_Als_NextOverlayMode.IA_Als_NextOverlayMode"))
  (if (UserInterface|Viewport|IsinViewport (Variables|State|GetOverlayModeMenuWidget))
    (Default|SelectNextOverlayMode (Variables|State|GetOverlayModeMenuWidget))))

(event Input|EnhancedActionEvents|EnhancedInputActionIA_Als_PreviousOverlayMode
  (params (ActionValue :type Boolean) (ElapsedSeconds :type Float%20%28double-precision%29) (TriggeredSeconds :type Float%20%28double-precision%29) (InputAction :type Input%20Action%20Object%20Reference :default "/ALS/Game/Data/Input/UI/IA_Als_PreviousOverlayMode.IA_Als_PreviousOverlayMode"))
  (if (UserInterface|Viewport|IsinViewport (Variables|State|GetOverlayModeMenuWidget))
    (Default|SelectPreviousOverlayMode (Variables|State|GetOverlayModeMenuWidget))))

(event Input|EnhancedActionEvents|EnhancedInputActionIA_Als_ToggleUI
  (params (ActionValue :type Boolean) (ElapsedSeconds :type Float%20%28double-precision%29) (TriggeredSeconds :type Float%20%28double-precision%29) (InputAction :type Input%20Action%20Object%20Reference :default "/ALS/Game/Data/Input/UI/IA_Als_ToggleUI.IA_Als_ToggleUI"))
  (Variables|State|SetbUIVisible (not (Variables|State|GetbUIVisible))))

(event Input|EnhancedActionEvents|EnhancedInputActionIA_Als_Slomo
  (params (ActionValue :type Boolean) (ElapsedSeconds :type Float%20%28double-precision%29) (TriggeredSeconds :type Float%20%28double-precision%29) (InputAction :type Input%20Action%20Object%20Reference :default "/ALS/Game/Data/Input/UI/IA_Als_Slomo.IA_Als_Slomo"))
  (Variables|State|SetbSlomoActive (not (Variables|State|GetbSlomoActive)))
  (CallFunction|SetGlobalTimeDilation (Math|Float|SelectFloat 0.15 1.0 (Variables|State|GetbSlomoActive))))

(event EventBeginPlay
  (if (Pawn|IsLocalController)
    (Input|SetInputModeGameOnly self false)
    (Input|AddMappingContext (PlayerController|LocalPlayerSubsystems|GetEnhancedInputLocalPlayerSubsystem) "/ALS/Game/Data/Input/IMC_Als_UI.IMC_Als_UI" 0 "(bIgnoreAllPressedKeysUntilRelease=True,bForceImmediately=False,bNotifyUserSettings=False)")
    (bind _returnvalue (UserInterface|CreateWidget "/ALS/Game/Art/UI/W_Als_Hud.W_Als_Hud_C" self))
    (UserInterface|Viewport|AddtoViewport _returnvalue 0)
    (bind _returnvalue_2 (UserInterface|CreateWidget "/ALS/Game/Art/UI/W_Als_OverlayModeMenu.W_Als_OverlayModeMenu_C" self))
    (Variables|State|SetOverlayModeMenuWidget _returnvalue_2)))

(fn ConstructionScript)

(fn SetGlobalTimeDilation
  (params (Time%20Dilation :type Float%20%28double-precision%29))
  (if (Class|KismetSystemLibrary|IsStandalone)
    (Utilities|Time|SetGlobalTimeDilation Time%20Dilation)))